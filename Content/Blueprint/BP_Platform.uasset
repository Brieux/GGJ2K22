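; Color-coded platform that indexes into a generator's platform list and finds the closest platform of each color.
; Colored applies the cylinder material matching the Color enum.
; Four near-duplicate Nearest events search forward, then backward, from the platform's ID with modulo wraparound, calling themselves recursively to store ClosestRed, Blue, Yellow and Green references.
; Random color selection in the construction script is disconnected.
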(event `Colored`
  (bind _cylinder (`self.Cylinder`))
  (switch `/Game/Enum/Enum_Color` (`self.Color`)
    (:`NewEnumerator0`
      (`PrimitiveComponent.SetMaterial` _cylinder 0 "/Game/Material/M_Red.M_Red"))
    (:`NewEnumerator1`
      (`PrimitiveComponent.SetMaterial` _cylinder 0 "/Game/Material/M_Blue.M_Blue"))
    (:`NewEnumerator2`
      (`PrimitiveComponent.SetMaterial` _cylinder 0 "/Game/Material/M_Yellow.M_Yellow"))
    (:`NewEnumerator3`
      (`PrimitiveComponent.SetMaterial` _cylinder 0 "/Game/Material/M_Green.M_Green"))))

(event `Nearest Blue`
  (bind _generatorref (`self.GeneratorRef`))
  (bind _generatorref_2 (`self.GeneratorRef`))
  (bind _generatorref_3 (`self.GeneratorRef`))
  (bind _returnvalue (- (`self.ID`) (`self.Distance-`)))
  (bind _nbofobject (`/Game/Blueprint/BP_Generator.NBofObject` _generatorref))
  (bind _returnvalue_2 (mod (+ (`self.ID`) (`self.Distance-`)) (`/Game/Blueprint/BP_Generator.NBofObject` (`self.GeneratorRef`))))
  (if (`self.Find?`)
    (if (<= (`self.Distance+`) (`self.Distance-`))
      (set `self.ClosestBlue` (`|GetArrayItem` (`/Game/Blueprint/BP_Generator.ListPlatform` _generatorref_2) (mod (+ (`self.ID`) (`self.Distance+`)) (`/Game/Blueprint/BP_Generator.NBofObject` _generatorref_2))))
      (set `self.Init?` true)
      (set `self.Find?` false)
      (elif (< _returnvalue 0)
        (set `self.ClosestBlue` (`|GetArrayItem` (`/Game/Blueprint/BP_Generator.ListPlatform` _generatorref_3) (- (`/Game/Blueprint/BP_Generator.NBofObject` _generatorref_3) (`KismetMathLibrary.Abs_Int` _returnvalue))))
        (set `self.Init?` true)
        (set `self.Find?` false)
        (else
          (set `self.ClosestBlue` (`|GetArrayItem` (`/Game/Blueprint/BP_Generator.ListPlatform` (`self.GeneratorRef`)) _returnvalue))
          (set `self.Init?` true)
          (set `self.Find?` false))))
    (else
      (if (`self.Init?`)
        (set `self.Find?` false)
        (set `self.Sens+?` true)
        (set `self.Distance+` 1)
        (set `self.Distance-` _nbofobject)
        (set `self.Init?` false))
      (if (`self.Sens+?`)
        (if (`|EnumEquality` (`/Game/Blueprint/BP_Platform.Color` (`|GetArrayItem` (`/Game/Blueprint/BP_Generator.ListPlatform` _generatorref) (mod (+ (`self.Distance+`) (`self.ID`)) _nbofobject))) "NewEnumerator1")
          (set `self.Sens+?` false)
          (else
            (set `self.Distance+` (+ (`self.Distance+`) 1))))
        (elif (== _returnvalue_2 (`self.ID`))
          (set `self.Distance-` (- (`self.Distance-`) 1) :!label _label)
          (elif (`|EnumEquality` (`/Game/Blueprint/BP_Platform.Color` (`|GetArrayItem` (`/Game/Blueprint/BP_Generator.ListPlatform` (`self.GeneratorRef`)) _returnvalue_2)) "NewEnumerator1")
            (set `self.Distance-` (- (`/Game/Blueprint/BP_Generator.NBofObject` (`self.GeneratorRef`)) (`self.Distance-`)))
            (set `self.Find?` true)
            (else
              (goto _label)))))
      (`self.Nearest Blue`))))

(event `NearestRed`
  (bind _generatorref (`self.GeneratorRef`))
  (bind _generatorref_2 (`self.GeneratorRef`))
  (bind _generatorref_3 (`self.GeneratorRef`))
  (bind _returnvalue (- (`self.ID`) (`self.Distance-`)))
  (bind _nbofobject (`/Game/Blueprint/BP_Generator.NBofObject` _generatorref))
  (bind _returnvalue_2 (mod (+ (`self.ID`) (`self.Distance-`)) (`/Game/Blueprint/BP_Generator.NBofObject` (`self.GeneratorRef`))))
  ;[1 1 1] nearRed
  (if (`self.Find?`)
    (if (<= (`self.Distance+`) (`self.Distance-`))
      (set `self.ClosestRed` (`|GetArrayItem` (`/Game/Blueprint/BP_Generator.ListPlatform` _generatorref_2) (mod (+ (`self.ID`) (`self.Distance+`)) (`/Game/Blueprint/BP_Generator.NBofObject` _generatorref_2))))
      (set `self.Find?` false)
      (set `self.Init?` true)
      (elif (< _returnvalue 0)
        (set `self.ClosestRed` (`|GetArrayItem` (`/Game/Blueprint/BP_Generator.ListPlatform` _generatorref_3) (- (`/Game/Blueprint/BP_Generator.NBofObject` _generatorref_3) (`KismetMathLibrary.Abs_Int` _returnvalue))))
        (set `self.Find?` false)
        (set `self.Init?` true)
        (else
          (set `self.ClosestRed` (`|GetArrayItem` (`/Game/Blueprint/BP_Generator.ListPlatform` (`self.GeneratorRef`)) _returnvalue))
          (set `self.Find?` false)
          (set `self.Init?` true))))
    (else
      (if (`self.Init?`)
        (set `self.Sens+?` true)
        (set `self.Find?` false)
        (set `self.Distance+` 1)
        (set `self.Distance-` _nbofobject)
        (set `self.Init?` false))
      (if (`self.Sens+?`)
        (if (`|EnumEquality` (`/Game/Blueprint/BP_Platform.Color` (`|GetArrayItem` (`/Game/Blueprint/BP_Generator.ListPlatform` _generatorref) (mod (+ (`self.Distance+`) (`self.ID`)) _nbofobject))) "NewEnumerator0")
          (set `self.Sens+?` false)
          (`self.NearestRed`)
          (else
            (set `self.Distance+` (+ (`self.Distance+`) 1))
            (`self.NearestRed`)))
        (elif (== _returnvalue_2 (`self.ID`))
          (set `self.Distance-` (- (`self.Distance-`) 1) :!label _label_2)
          (`self.NearestRed`)
          (elif (`|EnumEquality` (`/Game/Blueprint/BP_Platform.Color` (`|GetArrayItem` (`/Game/Blueprint/BP_Generator.ListPlatform` (`self.GeneratorRef`)) _returnvalue_2)) "NewEnumerator0")
            (set `self.Distance-` (- (`/Game/Blueprint/BP_Generator.NBofObject` (`self.GeneratorRef`)) (`self.Distance-`)))
            (set `self.Find?` true)
            (`self.NearestRed`)
            (else
              (goto _label_2))))))))

(event `NearestYellow`
  (bind _generatorref (`self.GeneratorRef`))
  (bind _generatorref_2 (`self.GeneratorRef`))
  (bind _generatorref_3 (`self.GeneratorRef`))
  (bind _returnvalue (- (`self.ID`) (`self.Distance-`)))
  (bind _nbofobject (`/Game/Blueprint/BP_Generator.NBofObject` _generatorref))
  (bind _returnvalue_2 (mod (+ (`self.ID`) (`self.Distance-`)) (`/Game/Blueprint/BP_Generator.NBofObject` (`self.GeneratorRef`))))
  (if (`self.Find?`)
    (if (<= (`self.Distance+`) (`self.Distance-`))
      (set `self.ClosestYellow` (`|GetArrayItem` (`/Game/Blueprint/BP_Generator.ListPlatform` _generatorref_2) (mod (+ (`self.ID`) (`self.Distance+`)) (`/Game/Blueprint/BP_Generator.NBofObject` _generatorref_2))))
      (set `self.Init?` true)
      (set `self.Find?` false)
      (elif (< _returnvalue 0)
        (set `self.ClosestYellow` (`|GetArrayItem` (`/Game/Blueprint/BP_Generator.ListPlatform` _generatorref_3) (- (`/Game/Blueprint/BP_Generator.NBofObject` _generatorref_3) (`KismetMathLibrary.Abs_Int` _returnvalue))))
        (set `self.Init?` true)
        (set `self.Find?` false)
        (else
          (set `self.ClosestYellow` (`|GetArrayItem` (`/Game/Blueprint/BP_Generator.ListPlatform` (`self.GeneratorRef`)) _returnvalue))
          (set `self.Init?` true)
          (set `self.Find?` false))))
    (else
      (if (`self.Init?`)
        (set `self.Find?` false)
        (set `self.Sens+?` true)
        (set `self.Distance+` 1)
        (set `self.Distance-` _nbofobject)
        (set `self.Init?` false))
      (if (`self.Sens+?`)
        (if (`|EnumEquality` (`/Game/Blueprint/BP_Platform.Color` (`|GetArrayItem` (`/Game/Blueprint/BP_Generator.ListPlatform` _generatorref) (mod (+ (`self.Distance+`) (`self.ID`)) _nbofobject))) "NewEnumerator2")
          (set `self.Sens+?` false)
          (else
            (set `self.Distance+` (+ (`self.Distance+`) 1))))
        (elif (== _returnvalue_2 (`self.ID`))
          (set `self.Distance-` (- (`self.Distance-`) 1) :!label _label_3)
          (elif (`|EnumEquality` (`/Game/Blueprint/BP_Platform.Color` (`|GetArrayItem` (`/Game/Blueprint/BP_Generator.ListPlatform` (`self.GeneratorRef`)) _returnvalue_2)) "NewEnumerator2")
            (set `self.Distance-` (- (`/Game/Blueprint/BP_Generator.NBofObject` (`self.GeneratorRef`)) (`self.Distance-`)))
            (set `self.Find?` true)
            (else
              (goto _label_3)))))
      (`self.NearestYellow`))))

(event `NearestGreen`
  (bind _generatorref (`self.GeneratorRef`))
  (bind _generatorref_2 (`self.GeneratorRef`))
  (bind _generatorref_3 (`self.GeneratorRef`))
  (bind _returnvalue (- (`self.ID`) (`self.Distance-`)))
  (bind _nbofobject (`/Game/Blueprint/BP_Generator.NBofObject` _generatorref))
  (bind _returnvalue_2 (mod (+ (`self.ID`) (`self.Distance-`)) (`/Game/Blueprint/BP_Generator.NBofObject` (`self.GeneratorRef`))))
  (if (`self.Find?`)
    (if (<= (`self.Distance+`) (`self.Distance-`))
      (set `self.ClosestGreen` (`|GetArrayItem` (`/Game/Blueprint/BP_Generator.ListPlatform` _generatorref_2) (mod (+ (`self.ID`) (`self.Distance+`)) (`/Game/Blueprint/BP_Generator.NBofObject` _generatorref_2))))
      (set `self.Init?` true)
      (set `self.Find?` false)
      (elif (< _returnvalue 0)
        (set `self.ClosestGreen` (`|GetArrayItem` (`/Game/Blueprint/BP_Generator.ListPlatform` _generatorref_3) (- (`/Game/Blueprint/BP_Generator.NBofObject` _generatorref_3) (`KismetMathLibrary.Abs_Int` _returnvalue))))
        (set `self.Init?` true)
        (set `self.Find?` false)
        (else
          (set `self.ClosestGreen` (`|GetArrayItem` (`/Game/Blueprint/BP_Generator.ListPlatform` (`self.GeneratorRef`)) _returnvalue))
          (set `self.Init?` true)
          (set `self.Find?` false))))
    (else
      (if (`self.Init?`)
        (set `self.Find?` false)
        (set `self.Sens+?` true)
        (set `self.Distance+` 1)
        (set `self.Distance-` _nbofobject)
        (set `self.Init?` false))
      (if (`self.Sens+?`)
        (if (`|EnumEquality` (`/Game/Blueprint/BP_Platform.Color` (`|GetArrayItem` (`/Game/Blueprint/BP_Generator.ListPlatform` _generatorref) (mod (+ (`self.Distance+`) (`self.ID`)) _nbofobject))) "NewEnumerator3")
          (set `self.Sens+?` false)
          (`self.NearestGreen`)
          (else
            (set `self.Distance+` (+ (`self.Distance+`) 1))
            (`self.NearestGreen`)))
        (elif (== _returnvalue_2 (`self.ID`))
          (set `self.Distance-` (- (`self.Distance-`) 1) :!label _label_4)
          (`self.NearestGreen`)
          (elif (`|EnumEquality` (`/Game/Blueprint/BP_Platform.Color` (`|GetArrayItem` (`/Game/Blueprint/BP_Generator.ListPlatform` (`self.GeneratorRef`)) _returnvalue_2)) "NewEnumerator3")
            (set `self.Distance-` (- (`/Game/Blueprint/BP_Generator.NBofObject` (`self.GeneratorRef`)) (`self.Distance-`)))
            (set `self.Find?` true)
            (`self.NearestGreen`)
            (else
              (goto _label_4))))))))

(fn `UserConstructionScript`)