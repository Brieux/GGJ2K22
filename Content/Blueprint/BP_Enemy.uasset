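; Golem enemy that hops around a looping set of platforms relative to the player, with a random speed type and color weakness.
; Speed picks mesh, animation and move countdown (type 0 stays still, type 3 jumps two platforms), while weakness sets the material.
; Tick runs the countdown unless stunned, then CalculMove chooses a direction from platform IDs and a timeline lerps the jump.
; Once DeadAvailable is set, it awards score, frees its platform and destroys itself.
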(event `Reset`
  (bind _skeletalmesh (`self.SkeletalMesh`))
  (switch `int` (`self.Speed`) :!label _label
    (:`0`
      (`SkinnedMeshComponent.SetSkinnedAssetAndUpdate` _skeletalmesh "/Game/Mesh/Golem/A_Immobile/A_Golem_Immobile_Idle.A_Golem_Immobile_Idle" true))
    (:`1`
      (`SkinnedMeshComponent.SetSkinnedAssetAndUpdate` _skeletalmesh "/Game/Mesh/Golem/A_Standard/A_Golem_Standard_Idle.A_Golem_Standard_Idle" true))
    (:`2`
      (`SkinnedMeshComponent.SetSkinnedAssetAndUpdate` _skeletalmesh "/Game/Mesh/Golem/A_LongueJambe/A_LJ_Idle.A_LJ_Idle" true))
    (:`3`
      (`SkinnedMeshComponent.SetSkinnedAssetAndUpdate` _skeletalmesh "/Game/Mesh/Golem/A_Long/A_Golem_Long_Idle.A_Golem_Long_Idle" true)))
  (`PrimitiveComponent.SetMaterial` _skeletalmesh 0 (select `/Game/Enum/Enum_Color` (`self.Faiblesse`) :`NewEnumerator0` "/Game/TestAnto/MatLavaToken.MatLavaToken" :`NewEnumerator1` "/Game/Material/M_Glace.M_Glace" :`NewEnumerator2` "/Game/Material/MatGolem/Mat_Sand.Mat_Sand" :`NewEnumerator3` "/Game/Material/MatGolem/Mat_Moss.Mat_Moss" :!type "MaterialInterface Object Reference"))
  (`SkeletalMeshComponent.SetAnimInstanceClass` (`self.SkeletalMesh`) (select `int` (`self.Speed`) :`0` "/Game/Mesh/Golem/A_Immobile/ABP_Golem_Immo.ABP_Golem_Immo_C" :`1` "/Game/Mesh/Golem/A_Standard/ABP_Golem_Standard.ABP_Golem_Standard_C" :`2` "/Game/Mesh/Golem/A_LongueJambe/ABP_LJ.ABP_LJ_C" :`3` "/Game/Mesh/Golem/A_Long/ABP_Golem_LJ.ABP_Golem_LJ_C" :!type "Object Class Reference")))

(event `self.ReceiveBeginPlay`
  (bind _output_get (set `self.Speed` (`KismetMathLibrary.RandomIntegerInRange` 0 3)))
  (set `self.TourDeJeu` _output_get)
  (set `self.Faiblesse` (cast `/Game/Enum/Enum_Color` (`KismetMathLibrary.Conv_IntToByte` (`KismetMathLibrary.RandomIntegerInRange` 0 3))))
  (bind _asbp_player (cast `/Game/Blueprint/BP_Player` (`Controller.K2_GetPawn` (`GameplayStatics.GetPlayerController` 0))))
  (set `self.As BP Player` _asbp_player)
  (goto _label))

(event `/Game/Int_Tickable.Tick`
  (if (not (== (`self.Speed`) 0))
    (if (== (`self.Speed`) 3)
      (set `self.Pas` 2))
    (if (`self.Stun?`)
      (set `self.Stun?` false)
      (elif (== (`self.TourDeJeu`) 0)
        (`self.CalculMove`)
        (set `self.TourDeJeu` (`self.Speed`))
        (else
          (set `self.TourDeJeu` (- (`self.TourDeJeu`) 1)))))))

(event `self.ReceiveTick`
  (params (DeltaSeconds :type "Float (single-precision)"))
  (bind _as_bp_player (`self.As BP Player`))
  (bind _platform (`self.Platform`))
  (if (`self.DeadAvailable`)
    (set `/Game/Blueprint/BP_Player.Score` (+ (`/Game/Blueprint/BP_Player.Score` _as_bp_player) 1) _as_bp_player)
    (set `/Game/Blueprint/BP_Platform.EnemyOnIt?` false _platform)
    (set `/Game/Blueprint/BP_Platform.Enemy` null _platform)
    (`self.K2_DestroyActor`)))

(event `CalculMove`
  (bind _platform (`self.Platform`))
  (if (== (mod (- (`/Game/Blueprint/BP_Platform.ID` _platform) (`/Game/Blueprint/BP_Platform.ID` (`/Game/Blueprint/BP_Player.newPlatform` (`self.As BP Player`)))) (/ (`/Game/Blueprint/BP_Generator.NBofObject` (`/Game/Blueprint/BP_Platform.GeneratorRef` _platform)) 2)) 0)
    (set `self.Equi` true)
    (`self.Movement`)
    (else
      (if (> (`/Game/Blueprint/BP_Platform.ID` (`self.Platform`)) (`/Game/Blueprint/BP_Platform.ID` (`/Game/Blueprint/BP_Player.newPlatform` (`self.As BP Player`))))
        (set `self.Distance+` (- (`/Game/Blueprint/BP_Generator.NBofObject` (`/Game/Blueprint/BP_Platform.GeneratorRef` (`self.Platform`))) (- (`/Game/Blueprint/BP_Platform.ID` (`/Game/Blueprint/BP_Player.newPlatform` (`self.As BP Player`))) (`/Game/Blueprint/BP_Platform.ID` (`self.Platform`)))))
        (else
          (set `self.Distance+` (- (`/Game/Blueprint/BP_Platform.ID` (`/Game/Blueprint/BP_Player.newPlatform` (`self.As BP Player`))) (`/Game/Blueprint/BP_Platform.ID` (`self.Platform`))))))
      (if (< (`/Game/Blueprint/BP_Platform.ID` (`self.Platform`)) (`/Game/Blueprint/BP_Platform.ID` (`/Game/Blueprint/BP_Player.newPlatform` (`self.As BP Player`))))
        (set `self.Distance-` (- (`/Game/Blueprint/BP_Generator.NBofObject` (`/Game/Blueprint/BP_Platform.GeneratorRef` (`self.Platform`))) (- (`/Game/Blueprint/BP_Platform.ID` (`/Game/Blueprint/BP_Player.newPlatform` (`self.As BP Player`))) (`/Game/Blueprint/BP_Platform.ID` (`self.Platform`)))))
        (else
          (set `self.Distance-` (- (`/Game/Blueprint/BP_Platform.ID` (`self.Platform`)) (`/Game/Blueprint/BP_Platform.ID` (`/Game/Blueprint/BP_Player.newPlatform` (`self.As BP Player`)))))))
      (if (> (`self.Distance+`) (`self.Distance-`))
        (set `self.Sens+?` false)
        (else
          (set `self.Sens+?` true)))
      (`self.Movement`))))

(event `Die`
  (set `self.TriggerDead` true))

(event `Movement`
  (bind _platform (`self.Platform`))
  (bind _generatorref (`/Game/Blueprint/BP_Platform.GeneratorRef` _platform))
  (bind _returnvalue (- (`/Game/Blueprint/BP_Platform.ID` (`self.Platform`)) (`self.Pas`)))
  (bind _listplatform (`/Game/Blueprint/BP_Generator.ListPlatform` (`/Game/Blueprint/BP_Platform.GeneratorRef` (`self.Platform`))))
  (if (`self.Equi`)
    (set `self.Sens+?` (`KismetMathLibrary.Conv_IntToBool` (`KismetMathLibrary.RandomIntegerInRange` 0 1))))
  (if (`self.Sens+?`)
    (set `self.NewPlatform` (`|GetArrayItem` (`/Game/Blueprint/BP_Generator.ListPlatform` _generatorref) (mod (+ (`/Game/Blueprint/BP_Platform.ID` _platform) (`self.Pas`)) (`/Game/Blueprint/BP_Generator.NBofObject` _generatorref))))
    (elif (< _returnvalue 0)
      (set `self.NewPlatform` (`|GetArrayItem` _listplatform (+ _returnvalue 30)))
      (else
        (set `self.NewPlatform` (`|GetArrayItem` _listplatform _returnvalue)))))
  (`self.DeplacementIG`))

(event `DeplacementIG`
  (bind _platform (`self.Platform`))
  (bind _sphere (`self.Sphere`))
  (set `self.initPos` (`SceneComponent.K2_GetComponentLocation` (`self.Sphere`)))
  (`TimelineComponent.SetPlayRate` (`self.Timeline_0`) 0.5)
  (set `self.triggerJump` true)
  (`KismetSystemLibrary.PrintString` "Hello")
  (bind (_direction _newtrack_0) (`Timeline|Timeline_0` :!via `PlayFromStart`)
    (:`Update`
      (`SceneComponent.K2_SetWorldLocation` _sphere (`KismetMathLibrary.VLerp` (`self.initPos`) (`SceneComponent.K2_GetComponentLocation` (`/Game/Blueprint/BP_Platform.PlayerPos` (`self.NewPlatform`))) _newtrack_0) false false)
      (`SceneComponent.K2_SetWorldRotation` _sphere (`KismetMathLibrary.FindLookAtRotation` (`SceneComponent.K2_GetComponentLocation` _sphere) (`SceneComponent.K2_GetComponentLocation` (`/Game/Blueprint/BP_Player.DefaultSceneRoot` (`self.As BP Player`)))) false false))
    (:`Finished`
      (set `/Game/Blueprint/BP_Platform.Enemy` null _platform)
      (set `/Game/Blueprint/BP_Platform.EnemyOnIt?` false _platform)
      (bind _output_get (set `self.Platform` (`self.NewPlatform`)))
      (set `/Game/Blueprint/BP_Platform.EnemyOnIt?` true _output_get)
      (set `/Game/Blueprint/BP_Platform.Enemy` self _output_get)
      (set `self.Equi` false)
      (set `self.Distance+` 0)
      (set `self.Distance-` 0)
      (set `self.Sens+?` false)
      (set `self.NewPlatform` null)
      (set `self.initPos` (`SceneComponent.K2_GetComponentLocation` (`self.Sphere`))))))

(fn `UserConstructionScript`)