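; BP_Spell is a spell actor cast on a platform, killing an enemy there whose weakness (Faiblesse) matches its own.
; BeginPlay tints the Niagara effect by Faiblesse, then runs one effect chosen by Modifier.
; Red recurses onto neighbor platforms after kills; Green stuns; Blue stuns or spawns an ice wall.
; Yellow slows and shoves neighboring enemies outward, killing slower blockers, using modulo indexing into the generator's platform list.
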(event `self.ReceiveBeginPlay`
  (switch `/Game/Enum/Enum_Color` (`self.Faiblesse`)
    (:`NewEnumerator0`
      (`FXSystemComponent.SetColorParameter` (`self.Niagara`) "SpellColor" (struct :`R` 3.0 :`A` 1.0)))
    (:`NewEnumerator1`
      (`FXSystemComponent.SetColorParameter` (`self.Niagara`) "SpellColor" (struct :`B` 3.0 :`A` 1.0)))
    (:`NewEnumerator2`
      (`FXSystemComponent.SetColorParameter` (`self.Niagara`) "SpellColor" (struct :`R` 3.0 :`G` 3.0 :`A` 1.0)))
    (:`NewEnumerator3`
      (`FXSystemComponent.SetColorParameter` (`self.Niagara`) "SpellColor" (struct :`G` 3.0 :`A` 1.0))))
  (switch `/Game/Enum/Enum_Color` (`self.Modifier`)
    (:`NewEnumerator0`
      (`self.RedSpell` (`self.RefPlateform`)))
    (:`NewEnumerator1`
      (`self.BlueSpell`))
    (:`NewEnumerator2`
      (`self.YellowSpell`))
    (:`NewEnumerator3`
      (`self.GreenSpell`))))

(event `GreenSpell`
  (bind _refplateform (`self.RefPlateform`))
  (bind _refplateform_2 (`self.RefPlateform`))
  (bind _generatorref (`/Game/Blueprint/BP_Platform.GeneratorRef` _refplateform))
  (bind _generatorref_2 (`/Game/Blueprint/BP_Platform.GeneratorRef` _refplateform_2))
  (bind _enemy (`/Game/Blueprint/BP_Platform.Enemy` (`self.RefPlateform`)))
  (bind _output (`|GetArrayItem` (`/Game/Blueprint/BP_Generator.ListPlatform` _generatorref) (mod (+ (`/Game/Blueprint/BP_Platform.ID` _refplateform) 1) (`/Game/Blueprint/BP_Generator.NBofObject` _generatorref))))
  (bind _output_2 (`|GetArrayItem` (`/Game/Blueprint/BP_Generator.ListPlatform` _generatorref_2) (- (`/Game/Blueprint/BP_Generator.NBofObject` _generatorref_2) (+ (`/Game/Blueprint/BP_Platform.ID` _refplateform_2) 1))))
  ;[0.04278 1 0] GreenSpell
  (if (`/Game/Blueprint/BP_Platform.EnemyOnIt?` (`self.RefPlateform`))
    (if (`|EnumEquality` (`/Game/Blueprint/BP_Enemy.Faiblesse` _enemy) (`self.Faiblesse`))
      (`/Game/Blueprint/BP_Enemy.Die` _enemy)
      (else
        (set `/Game/Blueprint/BP_Enemy.Stun?` true _enemy)))
    (else
      (if (`/Game/Blueprint/BP_Platform.EnemyOnIt?` _output)
        (set `/Game/Blueprint/BP_Enemy.Stun?` true (`/Game/Blueprint/BP_Platform.Enemy` _output)))
      (if (`/Game/Blueprint/BP_Platform.EnemyOnIt?` _output_2)
        (set `/Game/Blueprint/BP_Enemy.Stun?` true (`/Game/Blueprint/BP_Platform.Enemy` _output_2))))))

(event `BlueSpell`
  (bind _refplateform (`self.RefPlateform`))
  (bind _enemy (`/Game/Blueprint/BP_Platform.Enemy` (`self.RefPlateform`)))
  ;[0 0.5902 1] BlueSpell
  (if (`/Game/Blueprint/BP_Platform.EnemyOnIt?` _refplateform)
    (if (`|EnumEquality` (`/Game/Blueprint/BP_Enemy.Faiblesse` (`/Game/Blueprint/BP_Platform.Enemy` (`self.RefPlateform`))) (`self.Faiblesse`))
      (`/Game/Blueprint/BP_Enemy.Die` _enemy)
      (else
        (set `/Game/Blueprint/BP_Enemy.Stun?` true _enemy)))
    (else
      (`|SpawnActorFromClass` "/Game/Blueprint/BP_IceWall.BP_IceWall_C" (`KismetMathLibrary.MakeTransform` (`SceneComponent.K2_GetComponentLocation` (`/Game/Blueprint/BP_Platform.PlayerPos` _refplateform))) "Undefined" "OverrideRootScale" null null))))

(event `RedSpell`
  (params (ThisOne :type "/Game/Blueprint/BP_Platform Object Reference"))
  (bind _refplateform (`self.RefPlateform`))
  (bind _refplateform_2 (`self.RefPlateform`))
  (bind _enemy (`/Game/Blueprint/BP_Platform.Enemy` ThisOne))
  (bind _generatorref (`/Game/Blueprint/BP_Platform.GeneratorRef` _refplateform))
  (bind _generatorref_2 (`/Game/Blueprint/BP_Platform.GeneratorRef` _refplateform_2))
  ;[1 0.05263 0] RedSpell
  (if (`/Game/Blueprint/BP_Platform.EnemyOnIt?` ThisOne)
    (if (`|EnumEquality` (`/Game/Blueprint/BP_Enemy.Faiblesse` _enemy) (`self.Faiblesse`))
      (`/Game/Blueprint/BP_Enemy.Die` _enemy)
      (`self.RedSpell` (`|GetArrayItem` (`/Game/Blueprint/BP_Generator.ListPlatform` _generatorref_2) (mod (+ (`/Game/Blueprint/BP_Platform.ID` _refplateform_2) 1) (`/Game/Blueprint/BP_Generator.NBofObject` _generatorref_2))))
      (`self.RedSpell` (`|GetArrayItem` (`/Game/Blueprint/BP_Generator.ListPlatform` _generatorref) (- (`/Game/Blueprint/BP_Generator.NBofObject` _generatorref) (+ (`/Game/Blueprint/BP_Platform.ID` _refplateform) 1)))))))

(event `YellowSpell`
  (bind _refplateform (`self.RefPlateform`))
  (bind _refplateform_2 (`self.RefPlateform`))
  (bind _refplateform_3 (`self.RefPlateform`))
  (bind _refplateform_4 (`self.RefPlateform`))
  (bind _enemy (`/Game/Blueprint/BP_Platform.Enemy` (`self.RefPlateform`)))
  (bind _listplatform (`/Game/Blueprint/BP_Generator.ListPlatform` (`/Game/Blueprint/BP_Platform.GeneratorRef` _refplateform)))
  (bind _listplatform_2 (`/Game/Blueprint/BP_Generator.ListPlatform` (`/Game/Blueprint/BP_Platform.GeneratorRef` _refplateform_2)))
  (bind _listplatform_3 (`/Game/Blueprint/BP_Generator.ListPlatform` (`/Game/Blueprint/BP_Platform.GeneratorRef` _refplateform_3)))
  (bind _listplatform_4 (`/Game/Blueprint/BP_Generator.ListPlatform` (`/Game/Blueprint/BP_Platform.GeneratorRef` _refplateform_4)))
  (bind _output (`|GetArrayItem` _listplatform (mod (- (`/Game/Blueprint/BP_Platform.ID` _refplateform) 2) (`KismetArrayLibrary.Array_Length` _listplatform))))
  (bind _output_2 (`|GetArrayItem` _listplatform_2 (mod (- (`/Game/Blueprint/BP_Platform.ID` _refplateform_2) 1) (`KismetArrayLibrary.Array_Length` _listplatform_2))))
  (bind _output_3 (`|GetArrayItem` _listplatform_3 (mod (+ (`/Game/Blueprint/BP_Platform.ID` _refplateform_3) 1) (`KismetArrayLibrary.Array_Length` _listplatform_3))))
  (bind _output_4 (`|GetArrayItem` _listplatform_4 (mod (+ (`/Game/Blueprint/BP_Platform.ID` _refplateform_4) 2) (`KismetArrayLibrary.Array_Length` _listplatform_4))))
  (bind _enemy_2 (`/Game/Blueprint/BP_Platform.Enemy` _output_2))
  (bind _enemy_3 (`/Game/Blueprint/BP_Platform.Enemy` _output))
  (bind _enemy_4 (`/Game/Blueprint/BP_Platform.Enemy` _output_4))
  (bind _enemy_5 (`/Game/Blueprint/BP_Platform.Enemy` _output_3))
  ;[1 1 0] Yellow Spell
  (if (`/Game/Blueprint/BP_Platform.EnemyOnIt?` (`self.RefPlateform`))
    (if (`|EnumEquality` (`/Game/Blueprint/BP_Enemy.Faiblesse` (`/Game/Blueprint/BP_Platform.Enemy` (`self.RefPlateform`))) (`self.Faiblesse`))
      (`/Game/Blueprint/BP_Enemy.Die` (`/Game/Blueprint/BP_Platform.Enemy` (`self.RefPlateform`)))
      (else
        (set `/Game/Blueprint/BP_Enemy.Speed` (- (`/Game/Blueprint/BP_Enemy.Speed` _enemy) 1) _enemy))))
  (if (`/Game/Blueprint/BP_Platform.EnemyOnIt?` _output_3)
    (if (`/Game/Blueprint/BP_Platform.EnemyOnIt?` _output_4)
      (if (> (`/Game/Blueprint/BP_Enemy.Speed` (`/Game/Blueprint/BP_Platform.Enemy` _output_3)) (`/Game/Blueprint/BP_Enemy.Speed` _enemy_4))
        (`/Game/Blueprint/BP_Enemy.Die` _enemy_4)
        (set `/Game/Blueprint/BP_Enemy.Platform` _output_4 _enemy_5 :!label _label)
        (set `/Game/Blueprint/BP_Platform.EnemyOnIt?` false _output_3)
        (set `/Game/Blueprint/BP_Platform.Enemy` null _output_3)
        (set `/Game/Blueprint/BP_Platform.EnemyOnIt?` true _output_4)
        (set `/Game/Blueprint/BP_Platform.Enemy` _enemy_5 _output_4))
      (else
        (goto _label))))
  (if (`/Game/Blueprint/BP_Platform.EnemyOnIt?` _output_2)
    (if (`/Game/Blueprint/BP_Platform.EnemyOnIt?` _output)
      (if (> (`/Game/Blueprint/BP_Enemy.Speed` (`/Game/Blueprint/BP_Platform.Enemy` _output_2)) (`/Game/Blueprint/BP_Enemy.Speed` _enemy_3))
        (`/Game/Blueprint/BP_Enemy.Die` _enemy_3)
        (set `/Game/Blueprint/BP_Enemy.Platform` _output _enemy_2 :!label _label_2)
        (set `/Game/Blueprint/BP_Platform.EnemyOnIt?` false _output_2)
        (set `/Game/Blueprint/BP_Platform.Enemy` null _output_2)
        (set `/Game/Blueprint/BP_Platform.EnemyOnIt?` true _output)
        (set `/Game/Blueprint/BP_Platform.Enemy` _enemy_2 _output))
      (else
        (goto _label_2)))))

(fn `UserConstructionScript`)