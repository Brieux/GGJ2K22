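; Monster generator actor that spawns enemies onto platforms held by a referenced generator.
; SpawnEnemy picks a random platform index and calls itself again if that platform already has an enemy or is the player's platform.
; Otherwise it spawns a BP_Enemy at the platform's PlayerPos, then links enemy and platform to each other and flags the platform as occupied.
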(event `SpawnEnemy`
  (bind _refgenerator (`self.RefGenerator`))
  (bind _output (`|GetArrayItem` (`/Game/Blueprint/BP_Generator.ListPlatform` (`self.RefGenerator`)) (`self.NewVar_0`)))
  (set `self.NewVar_0` (`KismetMathLibrary.RandomIntegerInRange` 0 (`/Game/Blueprint/BP_Generator.NBofObject` _refgenerator)))
  (if (or (`/Game/Blueprint/BP_Platform.EnemyOnIt?` (`|GetArrayItem` (`/Game/Blueprint/BP_Generator.ListPlatform` _refgenerator) (`self.NewVar_0`))) (== (`/Game/Blueprint/BP_Platform.ID` (`/Game/Blueprint/BP_Player.newPlatform` (cast `/Game/Blueprint/BP_Player` (`Controller.K2_GetPawn` (`GameplayStatics.GetPlayerController` 0)) :!pure true))) (`self.NewVar_0`)))
    (`self.SpawnEnemy`)
    (else
      (bind _returnvalue (`|SpawnActorFromClass` "/Game/Blueprint/BP_Enemy.BP_Enemy_C" (`KismetMathLibrary.MakeTransform` (`SceneComponent.K2_GetComponentLocation` (`/Game/Blueprint/BP_Platform.PlayerPos` _output))) "Undefined" "OverrideRootScale" null null))
      (set `/Game/Blueprint/BP_Enemy.Platform` _output _returnvalue)
      (set `/Game/Blueprint/BP_Platform.EnemyOnIt?` true _output)
      (set `/Game/Blueprint/BP_Platform.Enemy` _returnvalue _output))))

(fn `UserConstructionScript`)