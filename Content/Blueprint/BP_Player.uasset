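; Player Blueprint that hops between colored platforms, with one input each for blue, green, yellow and red.
; Each input teleports it to that color's nearest platform, then caches the new platform's four closest neighbors.
; Each hop also records the platform color in a three-slot combo map (Plot, Faiblesse, Modifier).
; Once full, the map shifts entries up, keeping the last three colors as a sliding window.
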(event `TakeNearest`
  (params (NewPlatform :type "/Game/Blueprint/BP_Platform Object Reference"))
  ;[1 0.4679 0] SwitchNewPlatform
  (set `self.nearBlue` (`/Game/Blueprint/BP_Platform.ClosestBlue` NewPlatform))
  (set `self.nearGreen` (`/Game/Blueprint/BP_Platform.ClosestGreen` NewPlatform))
  (set `self.nearYellow` (`/Game/Blueprint/BP_Platform.ClosestYellow` NewPlatform))
  (set `self.nearRed` (`/Game/Blueprint/BP_Platform.ClosestRed` NewPlatform))
  (`self.AddToCombo`))

(event `InputAction|GoToYellow`
  (params (Key :type "Key Structure"))
  (bind _nearyellow (`self.nearYellow`))
  ;[1 0.1216 0] Deplacement
  (:`Pressed`
    (set `self.newPlatform` _nearyellow)
    (`SceneComponent.K2_SetWorldLocation` (`self.DefaultSceneRoot`) (`SceneComponent.K2_GetComponentLocation` (`/Game/Blueprint/BP_Platform.PlayerPos` _nearyellow)) false false)
    (`self.TakeNearest` _nearyellow)))

(event `InputAction|GoToBlue`
  (params (Key :type "Key Structure"))
  (bind _nearblue (`self.nearBlue`))
  ;[1 0.1216 0] Deplacement
  (:`Pressed`
    (set `self.newPlatform` _nearblue)
    (`SceneComponent.K2_SetWorldLocation` (`self.DefaultSceneRoot`) (`SceneComponent.K2_GetComponentLocation` (`/Game/Blueprint/BP_Platform.PlayerPos` _nearblue)) false false)
    (`self.TakeNearest` _nearblue)))

(event `InputAction|GoToGreen`
  (params (Key :type "Key Structure"))
  (bind _neargreen (`self.nearGreen`))
  ;[1 0.1216 0] Deplacement
  (:`Pressed`
    (set `self.newPlatform` _neargreen)
    (`SceneComponent.K2_SetWorldLocation` (`self.DefaultSceneRoot`) (`SceneComponent.K2_GetComponentLocation` (`/Game/Blueprint/BP_Platform.PlayerPos` _neargreen)) false false)
    (`self.TakeNearest` _neargreen)))

(event `AddToCombo`
  ;[0 0.1819 1] AddToCombo
  (if (`|EnumEquality` (`self.GateCombo`) "NewEnumerator0")
    (if (`self.End?`)
      (`self.RemonterCombo`)
      (else
        (set `self.End?` true)))
    (`BlueprintMapLibrary.Map_Add` (`self.ListeSort`) (`self.GateCombo`) (`/Game/Blueprint/BP_Platform.Color` (`self.newPlatform`)))
    (else
      (`BlueprintMapLibrary.Map_Add` (`self.ListeSort`) (`self.GateCombo`) (`/Game/Blueprint/BP_Platform.Color` (`self.newPlatform`)))
      (switch `/Game/Enum/Enum_Attaque` (`self.GateCombo`)
        (:`NewEnumerator1`
          (set `self.GateCombo` "NewEnumerator0"))
        (:`NewEnumerator2`
          (set `self.GateCombo` "NewEnumerator1"))))))

(event `InputAction|GoToRed`
  (params (Key :type "Key Structure"))
  (bind _nearred (`self.nearRed`))
  ;[1 0.1216 0] Deplacement
  (:`Pressed`
    (set `self.newPlatform` _nearred)
    (`SceneComponent.K2_SetWorldLocation` (`self.DefaultSceneRoot`) (`SceneComponent.K2_GetComponentLocation` (`/Game/Blueprint/BP_Platform.PlayerPos` _nearred)) false false)
    (`self.TakeNearest` _nearred)))

(event `RemonterCombo`
  ;[0 1 0.8682] Remonter
  (`BlueprintMapLibrary.Map_Add` (`self.ListeSort`) "NewEnumerator2" (`BlueprintMapLibrary.Map_Find` (`self.ListeSort`) "NewEnumerator1"))
  (`BlueprintMapLibrary.Map_Add` (`self.ListeSort`) "NewEnumerator1" (`BlueprintMapLibrary.Map_Find` (`self.ListeSort`) "NewEnumerator0")))

(event `StartingPos`
  (params (BeginPlatform :type "/Game/Blueprint/BP_Platform Object Reference"))
  ;[0 1 0.07112] InitPos
  (set `self.nearBlue` (`/Game/Blueprint/BP_Platform.ClosestBlue` BeginPlatform))
  (set `self.nearRed` (`/Game/Blueprint/BP_Platform.ClosestRed` BeginPlatform))
  (set `self.nearGreen` (`/Game/Blueprint/BP_Platform.ClosestGreen` BeginPlatform))
  (set `self.nearYellow` (`/Game/Blueprint/BP_Platform.ClosestYellow` BeginPlatform))
  (`SceneComponent.K2_SetWorldLocation` (`self.DefaultSceneRoot`) (`SceneComponent.K2_GetComponentLocation` (`/Game/Blueprint/BP_Platform.PlayerPos` BeginPlatform)) false false))

(fn `UserConstructionScript`)