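; BP_Generator builds a ring of colored BP_Platform actors at BeginPlay and starts the player on the first one.
; It rotates its root in even steps to place each platform, drawing colors randomly from a pool that refills when empty.
; Each platform then applies its color and runs nearest red, green, blue and yellow lookups.
; The construction script adjusts the platform count toward even divisions and sizes a radius preview sphere, hidden in play.
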(event `self.ReceiveBeginPlay`
  (bind _defaultsceneroot (`self.DefaultSceneRoot`))
  (bind _returnvalue (`SceneComponent.K2_GetComponentRotation` _defaultsceneroot))
  (`SceneComponent.SetVisibility` (`self.Sphere`) false false)
  (`SceneComponent.K2_SetWorldRotation` :`self` (`self.DefaultSceneRoot`))
  (for _index (range 1 (+ (`self.NBofObject`) 1))
    (bind _output_get (set `self.Ref` (`KismetArrayLibrary.Array_Random` (`self.Dispo`))))
    (`KismetArrayLibrary.Array_RemoveItem` (`self.Dispo`) _output_get)
    (bind _returnvalue_2 (`|SpawnActorFromClass` "/Game/Blueprint/BP_Platform.BP_Platform_C" (`KismetMathLibrary.MakeTransform` (0.0 0.0 0.0)) "Undefined" "OverrideRootScale" null _output_get self (- _index 1) null))
    (`self.K2_SetActorLocation` _returnvalue_2 (+ (`self.K2_GetActorLocation` _returnvalue_2) (* _returnvalue (* (`self.rayon`) 100.0))) false false)
    (`SceneComponent.K2_SetWorldRotation` _defaultsceneroot (`KismetMathLibrary.ComposeRotators` (`KismetMathLibrary.MakeRotator` 0.0 0.0 (`KismetMathLibrary.Conv_IntToDouble` (/ 360 (`self.NBofObject`)))) _returnvalue) false false)
    (`KismetArrayLibrary.Array_Add` (`self.ListPlatform`) _returnvalue_2)
    (if (`KismetArrayLibrary.Array_IsEmpty` (`self.Dispo`))
      (set `self.Dispo` (`self.DispoDefault`))))
  (for _array_element (`self.ListPlatform`)
    (`/Game/Blueprint/BP_Platform.Colored` _array_element)
    (`|ExecutionSequence`
      (:`then_0`
        (`/Game/Blueprint/BP_Platform.NearestRed` _array_element))
      (:`then_1`
        (`/Game/Blueprint/BP_Platform.NearestGreen` _array_element))
      (:`then_2`
        (`/Game/Blueprint/BP_Platform.Nearest Blue` _array_element))
      (:`then_3`
        (`/Game/Blueprint/BP_Platform.NearestYellow` _array_element))
      (:`then_4`
        (bind _asbp_player (cast `/Game/Blueprint/BP_Player` (`Controller.K2_GetPawn` (`GameplayStatics.GetPlayerController` 0))))
        (`/Game/Blueprint/BP_Player.StartingPos` _asbp_player (`|GetArrayItem` (`self.ListPlatform`)))))))

(fn `UserConstructionScript`
  (bind _nbofobject (`self.NBofObject`))
  (if (not (== (mod (`self.NBofObject`) 4) 0))
    (bind _output_get (set `self.NBofObject` (- (`KismetMathLibrary.Conv_IntToByte` (`self.NBofObject`)) (mod (`self.NBofObject`) 4)))))
  (if (not (== (mod 360 _output_get) 0))
    (set `self.NBofObject` (- (`KismetMathLibrary.Conv_IntToByte` _nbofobject) (mod 360 _nbofobject))))
  (`SceneComponent.SetRelativeScale3D` (`self.Sphere`) (`KismetMathLibrary.Conv_DoubleToVector` (* (`self.rayon`) 2.0))))